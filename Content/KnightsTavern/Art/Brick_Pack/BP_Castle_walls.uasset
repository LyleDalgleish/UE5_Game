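; BP_Castle_walls is a modular castle wall prop from the brick pack, with wall rows, pillars, arch, floor bricks, junk and a torch.
; The construction script runs a sequence that sets each component's visibility, propagated to children, from its own boolean, so each placed instance can be configured into a different wall variant.
; It has no active gameplay logic; the event stubs and extra function are empty.
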(event `self.ReceiveActorBeginOverlap`
  (params (OtherActor :type "Actor Object Reference")))

(fn `NewFunction_0`)

(fn `UserConstructionScript`
  (`|ExecutionSequence`
    (:`then_0`
      (`SceneComponent.SetVisibility` (`self.wall_2`) (`self.Row2_L`) true))
    (:`then_1`
      (`SceneComponent.SetVisibility` (`self.Floorbricks`) (`self.showFloorBrick`) true))
    (:`then_2`
      (`SceneComponent.SetVisibility` (`self.pillar_R`) (`self.showPillar_R`) true))
    (:`then_3`
      (`SceneComponent.SetVisibility` (`self.pillar_L`) (`self.showPillar_L`) true))
    (:`then_4`
      (`SceneComponent.SetVisibility` (`self.wall_2_side`) (`self.Row2_R`) true))
    (:`then_5`
      (`SceneComponent.SetVisibility` (`self.w2`) (`self.show_wall2`) true))
    (:`then_6`
      (`SceneComponent.SetVisibility` (`self.Junk_L`) (`self.ShowJunk_L`) true))
    (:`then_7`
      (`SceneComponent.SetVisibility` (`self.Junk_2ndWoe_L`) (`self.Junk_row2`) true))
    (:`then_8`
      (`SceneComponent.SetVisibility` (`self.SM_broke_wall_L`) (`self.Base_wall_L`) true))
    (:`then_9`
      (`SceneComponent.SetVisibility` (`self.SM_broke_wall_R`) (`self.Base_wall_R`) true))
    (:`then_10`
      (`SceneComponent.SetVisibility` (`self.wall_2_side1`) (`self.show_wall2_R`) true))
    (:`then_11`
      (`SceneComponent.SetVisibility` (`self.torch`) (`self.showTorch`) true))
    (:`then_12`
      (`SceneComponent.SetVisibility` (`self.Arch`) (`self.show_arch`) true))))